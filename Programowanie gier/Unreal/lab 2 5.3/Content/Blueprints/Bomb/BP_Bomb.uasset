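; BP_Bomb is a bomb actor that explodes when a linked trigger is activated.
; On BeginPlay it binds to the interaction event of the BP_Interaction component on its Trigger, if valid.
; An active interaction state detonates it, spawning a Niagara explosion at the bomb mesh, applying full radial damage around it and destroying the actor.
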(event Custom|OnInteraction
  (params (InteractionState :type Boolean))
  (if InteractionState
    (CallFunction|DetonateBomb)))

(event Custom|DetonateBomb
  (bind _bomb (Variables|Default|GetBomb))
  (bind _returnvalue (Transformation|GetWorldLocation _bomb))
  (Niagara|SpawnSystematLocation "/Game/FX/Explosion/NS_Explosion.NS_Explosion" _returnvalue)
  (Game|Damage|ApplyRadialDamage 1e+02 _returnvalue 1.5e+02 0 0 self 0 true "ECC_Visibility")
  (Actor|DestroyActor))

(event EventBeginPlay
  (bind _trigger (Variables|Default|GetTrigger))
  (if (Utilities|IsValid _trigger)
    (EventDispatchers|BindEventtoOnInteraction (Actor|GetComponentbyClass _trigger "/Game/Blueprints/InteractionSystem/BP_Interaction.BP_Interaction_C") (delegate Custom|OnInteraction))))

(fn ConstructionScript)