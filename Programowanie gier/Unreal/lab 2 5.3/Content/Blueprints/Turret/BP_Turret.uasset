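; Sentry turret that tracks the player character on sight and fires twin projectiles from two arrows until an interaction on its linked terminal deactivates it.
; PawnSensing runs at FireInterval, and each sighting flags the player as seen for just under one interval before firing.
; While flagged, Tick smoothly rotates the base in yaw and the turret mesh in clamped pitch toward the target.
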(event OnSeePawn(PawnSensing)
  (params (Pawn :type Pawn%20Object%20Reference))
  (if (Variables|Default|GetActive)
    (bind _asbp_third_person_character (Utilities|Casting|CastToBP_ThirdPersonCharacter Pawn))
    (Variables|Default|SetTarget _asbp_third_person_character)
    (Variables|Default|SetIsPlayerSeen true)
    (Utilities|FlowControl|Delay (- (Variables|/Script/AIModule.PawnSensingComponent|GetSensingInterval (Variables|Default|GetPawnSensing)) (Class|Actor|GetActorTickInterval)))
    (Variables|Default|SetIsPlayerSeen false)
    (CallFunction|UpdateFire)))

(event Custom|OnInteraction
  (params (InteractionState :type Boolean))
  (if InteractionState
    (Variables|Default|SetActive false)))

(event EventBeginPlay
  (bind _terminal (Variables|Default|GetTerminal))
  (Utilities|IsValid _terminal
    (:Is%20Valid
      (EventDispatchers|BindEventtoOnInteraction (Actor|GetComponentbyClass _terminal "/Game/Blueprints/InteractionSystem/BP_Interaction.BP_Interaction_C") (delegate Custom|OnInteraction)))))

(event EventTick
  (params (DeltaSeconds :type Float%20%28single-precision%29))
  (if (Variables|Default|GetIsPlayerSeen)
    (Utilities|IsValid (Variables|Default|GetTarget)
      (:Is%20Valid
        (CallFunction|UpdateRotation)))))

(fn ConstructionScript
  (Class|PawnSensingComponent|SetSensingInterval (Variables|Default|GetPawnSensing) (Variables|Default|GetFireInterval)))

(fn UpdateRotation
  (bind _returnvalue (Utilities|Time|GetWorldDeltaSeconds))
  (bind _sm_turret (Variables|Default|GetSM_Turret))
  (bind _target (Variables|Default|GetTarget))
  (bind _returnvalue_2 (Transformation|GetActorLocation _target))
  (bind _returnvalue_3 (Transformation|GetWorldLocation _sm_turret))
  (bind _returnvalue_4 (Transformation|GetWorldRotation _sm_turret))
  (bind _returnvalue_5 (Math|Rotator|FindLookatRotation _returnvalue_3 _returnvalue_2))
  (bind _returnvalue_6 (Math|Interpolation|RInterpTo _returnvalue_4 _returnvalue_5 _returnvalue 2.0))
  (Transformation|SetWorldRotation (Variables|Default|GetSM_TurretBase) (Math|Rotator|MakeRotator 0.0 0.0 (.yaw _returnvalue_6)) false false)
  (Transformation|SetRelativeRotation (Variables|Default|GetSM_Turret) (Math|Rotator|MakeRotator 0.0 (Math|Float|ClampAngle (.pitch _returnvalue_6) -45.0 3e+01) 0.0) false false))

(fn UpdateFire
  (Game|SpawnActorfromClass "/Game/Blueprints/Projectile/BP_Projectile.BP_Projectile_C" (Transformation|GetWorldTransform (Variables|Default|GetArrowL)) "Undefined" 0 0)
  (Game|SpawnActorfromClass "/Game/Blueprints/Projectile/BP_Projectile.BP_Projectile_C" (Transformation|GetWorldTransform (Variables|Default|GetArrowR)) "Undefined" 0 0))