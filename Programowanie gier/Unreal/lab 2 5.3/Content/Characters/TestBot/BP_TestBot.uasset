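; BP_TestBot is an AI test character that takes over the first player's view on start and carries a spline path, optionally closed into a loop during construction.
; BeginPlay sets the walk speed and detaches the path so it stays fixed in the world.
; When its ElementsDetector overlaps a Destructible object, it sets the blackboard's BombState to SpawnBomb, leaving the bomb logic outside this Blueprint.
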(event OnComponentBeginOverlap(ElementsDetector)
  (params (OverlappedComponent :type Primitive%20Component%20Object%20Reference) (OtherActor :type Actor%20Object%20Reference) (OtherComp :type Primitive%20Component%20Object%20Reference) (OtherBodyIndex :type Integer) (bFromSweep :type Boolean) (SweepResult :type Hit%20Result%20Structure%20%28by%20ref%29))
  (if (Utilities|Enum|Equal(Enum) (Collision|GetCollisionObjectType OtherComp) "ECC_Destructible")
    (Development|PrintString "Bomb it")
    (Class|BlackboardComponent|SetValueasName (AI|GetBlackboard 0) (Utilities|Name|MakeLiteralName "BombState") "SpawnBomb")))

(event EventBeginPlay
  (Variables|/Script/Engine.CharacterMovementComponent|SetMaxWalkSpeed (Variables|Character|GetCharacterMovement) (Variables|Default|GetWalkSpeed))
  (Transformation|DetachFromComponent (Variables|Default|GetMovementPath) "KeepWorld" "KeepWorld" "KeepWorld" true)
  (Game|Player|SetViewTargetwithBlend (Game|GetPlayerController 0) (Components|GetOwner (Variables|Camera|GetCamera)) 0.0 "VTBlend_Linear" 0.0 false))

(fn ConstructionScript
  (if (Variables|Default|GetPathIsClosedLoop)
    (Spline|SetClosedLoop (Variables|Default|GetMovementPath) true true)))