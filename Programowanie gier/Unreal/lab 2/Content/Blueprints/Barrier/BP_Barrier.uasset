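; BP_Barrier is a blinking laser barrier that dissolves the player character on contact.
; A looping timer started on BeginPlay toggles the visibility of the Box and its children, enabling or disabling Box collision to match.
; When an actor begins overlapping the Box, it is cast to BP_ThirdPersonCharacter and its Dissolve function is called.
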(event OnComponentBeginOverlap(Box)
  (params (OverlappedComponent :type Primitive%20Component%20Object%20Reference) (OtherActor :type Actor%20Object%20Reference) (OtherComp :type Primitive%20Component%20Object%20Reference) (OtherBodyIndex :type Integer) (bFromSweep :type Boolean) (SweepResult :type Hit%20Result%20Structure%20%28by%20ref%29))
  (bind _asbp_third_person_character (Utilities|Casting|CastToBP_ThirdPersonCharacter OtherActor))
  (Default|Dissolve _asbp_third_person_character))

(event Custom|ToggleLaser
  (bind _box (Variables|Default|GetBox))
  (Rendering|ToggleVisibility _box true)
  (Collision|SetCollisionEnabled (Variables|Default|GetBox) (select (Variables|/Script/Engine.SceneComponent|GetbVisible _box) "QueryAndPhysics" "NoCollision")))

(event EventBeginPlay
  (Utilities|Time|SetTimerbyEvent (delegate Custom|ToggleLaser) (Variables|Default|GetTimerInterval) true))

(fn ConstructionScript)