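; BP_Elevator is an elevator that moves between a start and an end position when BP_ThirdPersonCharacter or BP_TestBot overlaps its Box component.
; The IsAtStart flag picks the direction, stopping the opposite MoveComponentTo before starting an eased, timed move of the Box.
; Each completed move updates the flag and prints a debug string.
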(event OnComponentBeginOverlap(Box)
  (params (OverlappedComponent :type Primitive%20Component%20Object%20Reference) (OtherActor :type Actor%20Object%20Reference) (OtherComp :type Primitive%20Component%20Object%20Reference) (OtherBodyIndex :type Integer) (bFromSweep :type Boolean) (SweepResult :type Hit%20Result%20Structure%20%28by%20ref%29))
  (bind _box (Variables|Default|GetBox))
  (Utilities|Casting|CastToBP_ThirdPersonCharacter OtherActor
    (:then
      _)
    (:CastFailed
      (Utilities|Casting|CastToBP_TestBot OtherActor)))
  (if (Variables|Default|GetIsAtStart)
    (Utilities|FlowControl|Sequence
      (:then_0
        (goto _label_2 Stop))
      (:then_1
        (Components|MoveComponentTo _box (Variables|Default|GetEndPosition) "0, 0, 0" true true (Variables|Default|GetTime) false :!label _label)
        (Variables|Default|SetIsAtStart false)
        (Development|PrintString "End")))
    (else
      (Utilities|FlowControl|Sequence
        (:then_0
          (goto _label Stop))
        (:then_1
          (Components|MoveComponentTo _box (Variables|Default|GetStartPosition) "0, 0, 0" true true (Variables|Default|GetTime) false :!label _label_2)
          (Variables|Default|SetIsAtStart true)
          (Development|PrintString "Start"))))))

(fn ConstructionScript)