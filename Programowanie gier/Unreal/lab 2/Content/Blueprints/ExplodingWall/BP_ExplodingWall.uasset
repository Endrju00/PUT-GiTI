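; Destructible Chaos wall that breaks apart when it takes any damage, then cleans up its debris.
; The construction script registers the left and right child-actor anchor fields as initialization fields on the Geometry Collection.
; Explode spawns a short-lived BP_Damage at the center destruction point.
; After a delay, a timeline drives the material's Alpha Threshold to fade the debris, then destroys the actor.
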(event Custom|Explode
  (bind _returnvalue (Game|SpawnActorfromClass "/Game/Blueprints/ExplodingWall/BP_Damage.BP_Damage_C" (Transformation|GetWorldTransform (Variables|Default|GetFS_CenterDestruction)) "Undefined" 0 0))
  (Actor|SetLifeSpan _returnvalue 0.5)
  (Utilities|FlowControl|Delay 2.0)
  (bind _fade_value (Timeline|Fade%20Debris Play)
    (:Update
      (Rendering|Material|SetScalarParameterValueonMaterials (Variables|Default|GetGeometryCollectionComponent) "Alpha Threshold" _fade_value))
    (:Finished
      (Actor|DestroyActor))))

(event Game|Damage|EventAnyDamage
  (params (Damage :type Float%20%28single-precision%29) (DamageType :type Damage%20Type%20Object%20Reference) (InstigatedBy :type Controller%20Object%20Reference) (DamageCauser :type Actor%20Object%20Reference))
  (CallFunction|Explode))

(fn ConstructionScript
  (bind _geometrycollectioncomponent (Variables|Default|GetGeometryCollectionComponent))
  (bind _initializationfields (Variables|/Script/GeometryCollectionEngine.GeometryCollectionComponent|GetInitializationFields _geometrycollectioncomponent))
  (Utilities|Array|Clear _initializationfields)
  (CallFunction|SetAnchors (Variables|Default|GetBP_Anchor_Left) _initializationfields)
  (CallFunction|SetAnchors (Variables|Default|GetBP_Anchor_Right) _initializationfields))

(fn SetAnchors
  (params (AnchorActor :type Child%20Actor%20Component%20Object%20Reference) (TargetArray :type Array%20of%20Field%20System%20Actor%20Object%20References))
  (bind _asfs_anchor_field_generic (Utilities|Casting|CastToFS_AnchorField_Generic (Variables|/Script/Engine.ChildActorComponent|GetChildActor AnchorActor)))
  (Utilities|Array|Add TargetArray _asfs_anchor_field_generic))